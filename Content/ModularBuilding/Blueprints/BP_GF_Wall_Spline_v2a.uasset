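; Modular building wall actor that lines a spline with ground-floor meshes in the Construction Script.
; A seeded random stream, multiplied by a running instance counter, bounds the loop over the first floor's element array.
; Each looped element gets its own Hierarchical Instanced Static Mesh component, repeated along the whole spline.
; Spacing comes from mesh bounds plus an offset, and each instance faces the next spline point.
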(event EventBeginPlay)

(event Collision|EventActorBeginOverlap
  (params (OtherActor :type Actor%20Object%20Reference)))

(event EventTick
  (params (DeltaSeconds :type Float%20%28single-precision%29)))

(fn ConstructionScript
  (bind _floors_editor (Variables|Default|GetFLOORS%20EDITOR))
  (bind _output (Utilities|Array|Get(acopy) _floors_editor))
  (for _index (range 0 (Math|Random|RandomIntegerinRangefromStream 0 (Utilities|Array|LastIndex (.floorelements _output)) (Math|Random|MakeRandomStream (* (Variables|Default|GetInitial%20Random%20Seed) (Variables|Default|GetLoop%20Index)))))
    ;[0 0.08854 0.08236] v4
    (bind _returnvalue (AddComponent|AddHierarchicalInstancedStaticMeshComponent false (Variables|Default|GetRelative%20Transform)))
    (bind _output_get (Variables|Default|SetHierarchical%20Instanced%20Mesh _returnvalue))
    (Components|StaticMesh|SetStaticMesh _output_get (Utilities|Array|Get(acopy) (.floorelements _output) _index)) ; Ground Floor
    (bind _output_get_2 (Variables|Default|SetModule%20Width (Math|Float|Truncate (+ (.X (Math|Vector|BreakVector (- (.Max (Utilities|Struct|BreakBox (StaticMesh|GetBoundingBox (Utilities|Array|Get(acopy) (.floorelements _output) _index)))) (.Min (Utilities|Struct|BreakBox (StaticMesh|GetBoundingBox (Utilities|Array|Get(acopy) (.floorelements _output) _index))))))) (Variables|Default|GetDistance%20Offset)))))
    (bind _output_get_3 (Variables|Default|SetNumber%20of%20Instances (- (Math|Float|Floor (/ (Spline|GetSplineLength (Variables|Default|GetSpline)) _output_get_2)) 1)))
    (for _index_2 (range 0 _output_get_3)
      (Components|InstancedStaticMesh|AddInstance (Variables|Default|GetHierarchical%20Instanced%20Mesh) (Math|Transform|MakeTransform (CallFunction|GetLocationandIndex _index_2) (Math|Rotator|MakeRotfromX (- (CallFunction|GetLocationandIndex (+ _index_2 1)) (CallFunction|GetLocationandIndex _index_2)))) false)
      (Math|Integer|IncrementInt (Variables|Default|GetLoop%20Index)))))

(fn GetLocationandIndex
  (params (A :type Integer))
  (return (Spline|GetLocationatDistanceAlongSpline (Variables|Default|GetSpline) (* A (Variables|Default|GetModule%20Width)) "Local")))