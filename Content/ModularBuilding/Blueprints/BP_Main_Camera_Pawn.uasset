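; Camera pawn for the modular building creator, providing a mouse-driven free camera and a set of fixed views.
; On BeginPlay it gathers the isometric, front, back and side cameras into an array and adds the UI and camera widget to the viewport.
; Mouse axes drive controller yaw and pitch, while the wheel changes spring arm length within clamped limits.
; A height change event repositions the free camera's relative location.
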(event Custom|Camera_Height_Change
  (params (Height_Change :type Vector))
  (Transformation|SetRelativeLocation (Variables|Default|GetFree_Camera) Height_Change false false))

(event Custom|Generate%20Static%20Camera%20Array)

(event EventBeginPlay
  ;[1 1 1] Make Static Cameras Array and Display Bulding Creator UI
  (Variables|Default|SetBP_Static_Cameras_Array (Utilities|Array|MakeArray (Variables|Default|GetCamera_Isometric) (Variables|Default|GetCamera_Side_R) (Variables|Default|GetCamera_Back) (Variables|Default|GetCamera_Side_L) (Variables|Default|GetCamera_Front)))
  (bind _returnvalue (UserInterface|CreateWidget "/Game/ModularBuilding/Blueprints/BPW_UI_and_Cams.BPW_UI_and_Cams_C"))
  (UserInterface|Viewport|AddtoViewport _returnvalue 0))

(event Input|MouseEvents|MouseX
  (params (AxisValue :type Float%20%28single-precision%29))
  (bind _returnvalue (Pawn|GetControlRotation :!class /Script/Engine.Pawn))
  ;[1 1 1] Camera Move
  (Pawn|Input|AddControllerYawInput AxisValue)
  (Pawn|SetControlRotation (Game|GetPlayerController 0) (Math|Rotator|MakeRotator 0.0 (.pitch _returnvalue) (.yaw _returnvalue))))

(event Input|MouseEvents|MouseY
  (params (AxisValue :type Float%20%28single-precision%29))
  ;[1 1 1] Camera Move
  (Pawn|Input|AddControllerPitchInput AxisValue))

(event Input|MouseEvents|MouseWheelUp
  (params (Key :type Key%20Structure :default "None"))
  (bind _springarm (Variables|Default|GetSpringArm))
  ;[1 1 1] Camera Zoom In/Out
  (:Pressed
    (Variables|/Script/Engine.SpringArmComponent|SetTargetArmLength _springarm (Math|Float|Clamp(Float) (- (Variables|/Script/Engine.SpringArmComponent|GetTargetArmLength _springarm) (Variables|Default|GetZoom_Speed)) (Variables|Default|GetMin_Cam_Zoom) (Variables|Default|GetMax_Cam_Zoom)))))

(event Input|MouseEvents|MouseWheelDown
  (params (Key :type Key%20Structure :default "None"))
  (bind _springarm (Variables|Default|GetSpringArm))
  ;[1 1 1] Camera Zoom In/Out
  (:Pressed
    (Variables|/Script/Engine.SpringArmComponent|SetTargetArmLength _springarm (Math|Float|Clamp(Float) (+ (Variables|/Script/Engine.SpringArmComponent|GetTargetArmLength _springarm) (Variables|Default|GetZoom_Speed)) (Variables|Default|GetMin_Cam_Zoom) (Variables|Default|GetMax_Cam_Zoom)))))

(event Input|KeyboardEvents|W
  (params (Key :type Key%20Structure :default "None")))

(event Input|KeyboardEvents|S
  (params (Key :type Key%20Structure :default "None")))

(fn ConstructionScript)