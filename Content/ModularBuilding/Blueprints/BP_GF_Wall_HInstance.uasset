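; Modular building wall actor that builds a row of repeated mesh pieces in its construction script.
; Each RepeatingMeshCreator entry gets its own hierarchical instanced mesh component with a dynamic material on slot 0.
; Instances repeat NumInstances times along local Y, spaced by InstanceWidth from the entry's transform, printing the actor name for each.
; A simpler single-mesh debug path and plain instanced-mesh nodes remain disconnected; the event graph is empty.
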(event EventBeginPlay)

(event Collision|EventActorBeginOverlap
  (params (OtherActor :type Actor%20Object%20Reference)))

(event EventTick
  (params (DeltaSeconds :type Float%20%28single-precision%29)))

(fn ConstructionScript
  ;[0.5 0 0.1167] Structure Based Instancing
  (for _array_element (Variables|Default|GetRepeatingMeshCreator)
    (bind _returnvalue (AddComponent|AddHierarchicalInstancedStaticMeshComponent false))
    (bind _output_get (Variables|Default|SetHierarchical%20Instanced%20Mesh _returnvalue))
    (Components|StaticMesh|SetStaticMesh _output_get (.staticmesh _array_element))
    (bind _returnvalue_2 (Rendering|Material|CreateDynamicMaterialInstance (Variables|Default|GetHierarchical%20Instanced%20Mesh) 0 (.materialinstance _array_element) "None" :!class /Script/Engine.PrimitiveComponent))
    (Rendering|Material|SetMaterial (Variables|Default|GetHierarchical%20Instanced%20Mesh) 0 _returnvalue_2)
    (for _index (range 0 (- (Variables|Default|GetNumInstances) 1))
      (Components|InstancedStaticMesh|AddInstance (Variables|Default|GetHierarchical%20Instanced%20Mesh) (Math|Transform|MakeTransform (Math|Vector|MakeVector (.x (.Location (Math|Transform|BreakTransform (.transform _array_element)))) (+ (* _index (Variables|Default|GetInstance%20Width)) (.y (.Location (Math|Transform|BreakTransform (.transform _array_element))))) (.z (.Location (Math|Transform|BreakTransform (.transform _array_element))))) (.Rotation (Math|Transform|BreakTransform (.transform _array_element))) (.Scale (Math|Transform|BreakTransform (.transform _array_element)))) false)
      (Development|PrintString (Utilities|GetDisplayName 0)))))