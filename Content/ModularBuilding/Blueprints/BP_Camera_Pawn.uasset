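; Camera pawn for a modular building creator, with a free camera and an array of five static view cameras.
; BeginPlay fills that array and shows an info overlay, while M toggles the building customization widget and mouse cursor.
; Mouse axes steer control rotation with roll zeroed, the wheel zooms the spring arm within limits, and an event repositions the free camera.
; Menu-open checks and World Partition streaming activation are left unconnected.
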(event Custom|Camera_Height_Change
  (params (Height_Change :type Vector))
  (Transformation|SetRelativeLocation (Variables|Default|GetFree_Camera) Height_Change false false))

(event EventBeginPlay
  ;[0 0.2182 1] Make Static Cameras Array and Display UI Info Overlay
  (bind _returnvalue (UserInterface|CreateWidget "/Game/ModularBuilding/Blueprints/BPW_UI_Info_Overlay.BPW_UI_Info_Overlay_C"))
  (UserInterface|Viewport|AddtoViewport _returnvalue 0)
  (Variables|Default|SetBP_Static_Cameras_Array (Utilities|Array|MakeArray (Variables|Default|GetCamera_Isometric) (Variables|Default|GetCamera_Side_R) (Variables|Default|GetCamera_Back) (Variables|Default|GetCamera_Side_L) (Variables|Default|GetCamera_Front))))

(event Input|MouseEvents|MouseX
  (params (AxisValue :type Float%20%28single-precision%29))
  (bind _returnvalue (Pawn|GetControlRotation :!class /Script/Engine.Pawn))
  ;[0 1 0.1815] Camera Movement
  (Pawn|Input|AddControllerYawInput AxisValue)
  (Pawn|SetControlRotation (Game|GetPlayerController 0) (Math|Rotator|MakeRotator 0.0 (.pitch _returnvalue) (.yaw _returnvalue))) ; Split Structure Pin to expose Rotation Values
)

(event Input|MouseEvents|MouseY
  (params (AxisValue :type Float%20%28single-precision%29))
  ;[0 1 0.1815] Camera Movement
  (Pawn|Input|AddControllerPitchInput AxisValue))

(event Input|KeyboardEvents|M
  (params (Key :type Key%20Structure :default "None"))
  (bind _returnvalue (Game|GetPlayerController 0))
  ;[0.1329 0 1] Display Bulding Creator UI
  (:Pressed
    (Utilities|FlowControl|FlipFlop
      (:A
        (bind _returnvalue_2 (UserInterface|CreateWidget "/Game/ModularBuilding/Blueprints/BPW_UI_and_Cams.BPW_UI_and_Cams_C" _returnvalue))
        (bind _output_get (Variables|Default|SetBuilding%20Customize%20Widget _returnvalue_2))
        (UserInterface|Viewport|AddtoViewport _output_get 0)
        (Variables|/Script/Engine.PlayerController|SetbShowMouseCursor _returnvalue true) ; Show Cursor
        (Variables|Default|SetIs%20Menu%20Opened? true))
      (:B
        (bind _building_customize_widget (Variables|Default|GetBuilding%20Customize%20Widget) ; Get converted to Validate Get - will proceed only if Variable is assigned
          (:then
            (Widget|RemovefromParent _building_customize_widget)
            (Variables|/Script/Engine.PlayerController|SetbShowMouseCursor _returnvalue false) ; Hide Cursor
            (Variables|Default|SetIs%20Menu%20Opened? false))
          (:else))))))

(event Input|MouseEvents|MouseWheelUp
  (params (Key :type Key%20Structure :default "None"))
  (bind _springarm (Variables|Default|GetSpringArm))
  ;[0 0.1883 1] Camera Zoom In/Out
  (:Pressed
    (Variables|/Script/Engine.SpringArmComponent|SetTargetArmLength _springarm (Math|Float|Clamp(Float) (- (Variables|/Script/Engine.SpringArmComponent|GetTargetArmLength _springarm) (Variables|Default|GetZoom_Speed)) (Variables|Default|GetMin_Cam_Zoom) (Variables|Default|GetMax_Cam_Zoom)))))

(event Input|MouseEvents|MouseWheelDown
  (params (Key :type Key%20Structure :default "None"))
  (bind _springarm (Variables|Default|GetSpringArm))
  ;[0 0.1883 1] Camera Zoom In/Out
  (:Pressed
    (Variables|/Script/Engine.SpringArmComponent|SetTargetArmLength _springarm (Math|Float|Clamp(Float) (+ (Variables|/Script/Engine.SpringArmComponent|GetTargetArmLength _springarm) (Variables|Default|GetZoom_Speed)) (Variables|Default|GetMin_Cam_Zoom) (Variables|Default|GetMax_Cam_Zoom)))))

(event Input|KeyboardEvents|W
  (params (Key :type Key%20Structure :default "None")))

(event Input|KeyboardEvents|S
  (params (Key :type Key%20Structure :default "None")))

(fn ConstructionScript)