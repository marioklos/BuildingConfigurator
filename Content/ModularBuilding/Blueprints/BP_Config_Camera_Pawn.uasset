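; BP_Config_Camera_Pawn is a camera pawn in the ModularBuilding module, offering mouse look, zoom and height adjustment.
; MouseX and MouseY axes drive controller yaw and pitch, with the yaw path also forcing control-rotation roll to zero.
; Mouse wheel steps the spring arm length by ZoomSpeed within min/max limits.
; Camera_Height_Change sets the camera's relative location directly to the supplied value, without sweeping.
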(event Custom|Camera_Height_Change
  (params (Height_Change :type Vector))
  (Transformation|SetRelativeLocation (Variables|Default|GetCamera) Height_Change false false))

(event Input|MouseEvents|MouseX
  (params (AxisValue :type Float%20%28single-precision%29))
  (bind _returnvalue (Pawn|GetControlRotation :!class /Script/Engine.Pawn))
  ;[1 1 1] Camera Move
  (Pawn|Input|AddControllerYawInput AxisValue)
  (Pawn|SetControlRotation (Game|GetPlayerController 0) (Math|Rotator|MakeRotator 0.0 (.pitch _returnvalue) (.yaw _returnvalue))))

(event Input|MouseEvents|MouseY
  (params (AxisValue :type Float%20%28single-precision%29))
  ;[1 1 1] Camera Move
  (Pawn|Input|AddControllerPitchInput AxisValue))

(event Input|MouseEvents|MouseWheelUp
  (params (Key :type Key%20Structure :default "None"))
  (bind _springarm (Variables|Default|GetSpringArm))
  ;[1 1 1] Camera Zoom In/Out
  (:Pressed
    (Variables|/Script/Engine.SpringArmComponent|SetTargetArmLength _springarm (Math|Float|Clamp(Float) (- (Variables|/Script/Engine.SpringArmComponent|GetTargetArmLength _springarm) (Variables|Default|GetZoom_Speed)) (Variables|Default|GetMin_Cam_Zoom) (Variables|Default|GetMax_Cam_Zoom)))))

(event Input|MouseEvents|MouseWheelDown
  (params (Key :type Key%20Structure :default "None"))
  (bind _springarm (Variables|Default|GetSpringArm))
  ;[1 1 1] Camera Zoom In/Out
  (:Pressed
    (Variables|/Script/Engine.SpringArmComponent|SetTargetArmLength _springarm (Math|Float|Clamp(Float) (+ (Variables|/Script/Engine.SpringArmComponent|GetTargetArmLength _springarm) (Variables|Default|GetZoom_Speed)) (Variables|Default|GetMin_Cam_Zoom) (Variables|Default|GetMax_Cam_Zoom)))))

(event Input|KeyboardEvents|W
  (params (Key :type Key%20Structure :default "None")))

(event Input|KeyboardEvents|S
  (params (Key :type Key%20Structure :default "None")))

(fn ConstructionScript)