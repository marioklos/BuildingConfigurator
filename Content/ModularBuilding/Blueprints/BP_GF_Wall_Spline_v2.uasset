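; Modular building spline actor that builds ground-floor and first-floor wall modules along a spline in the construction script.
; Segments follow either spline points or ModuleWidth steps, optionally scaled or limited to full-length modules, with tangents clamped to avoid stretching.
; Each spline mesh picks a random mesh from its floor's creator array, seeded by seed times index for persistence.
; Only length-based placement shapes the raised first floor; the added HISM components receive no instances.
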(event EventBeginPlay)

(event Collision|EventActorBeginOverlap
  (params (OtherActor :type Actor%20Object%20Reference)))

(event EventTick
  (params (DeltaSeconds :type Float%20%28single-precision%29)))

(fn ConstructionScript
  (bind _spline (Variables|Default|GetSpline))
  (bind _ground_floor_creator (Variables|Default|GetGround%20Floor%20Creator))
  (bind _floor_creator (Variables|Default|GetFloor%20Creator))
  (bind _spline_2 (Variables|Default|GetSpline))
  (if (Variables|Default|GetAllow%20Scaling?) ; Allow Scaling?
    ;[1 1 1] Scale along the spline
    (Variables|Default|SetModule%20Width (Math|Float|Truncate (* (.x (Transformation|GetActorScale3D)) (Variables|Default|GetModule%20Width)))))
  (if (Variables|Default|GetSpline%20Points%20Placing?)
    ;[1 1 1] Spline Points Based Placing
    (for _index (range 0 (- (Spline|GetNumberOfSplinePoints (Variables|Default|GetSpline)) 1))
      (bind _output_get (Variables|Default|SetLoop%20Index _index))
      (bind _returnvalue (AddComponent|AddHierarchicalInstancedStaticMeshComponent true))
      (bind _output_get_2 (Variables|Default|SetHierarchical%20Instanced%20Mesh _returnvalue))
      (bind _returnvalue_2 (AddComponent|AddSplineMeshComponent (Components|GetOwner _output_get_2) false))
      (bind _returnvalue_3 (AddComponent|AddSplineMeshComponent (Components|GetOwner _output_get_2) false (Math|Transform|MakeTransform "0.000000,0.000000,300.000000" "0, 0, 0" "1.000000,1.000000,1.000000")))
      (Components|StaticMesh|SetStaticMesh _returnvalue_2 (Utilities|Array|Get(acopy) (.floorelements (Utilities|Array|Get(acopy) _ground_floor_creator (Math|Random|RandomIntegerinRangefromStream 0 (Utilities|Array|LastIndex _ground_floor_creator) (Math|Random|MakeRandomStream (* (Variables|Default|GetInitial%20Random%20Seed) (Variables|Default|GetLoop%20Index)))))))) ; Ground Floor
      (Components|StaticMesh|SetStaticMesh _returnvalue_3 (Utilities|Array|Get(acopy) (.floorelements (Utilities|Array|Get(acopy) _floor_creator (Math|Random|RandomIntegerinRangefromStream 0 (Utilities|Array|LastIndex _floor_creator) (Math|Random|MakeRandomStream (* (Variables|Default|GetInitial%20Random%20Seed) (Variables|Default|GetLoop%20Index)))))))) ; First Floor
      ;[0.3095 0 1] Open up the mesh, look at the pivot point gizmo to determine forward axis
      (SplineMesh|SetForwardAxis _returnvalue_2 "X" true)
      (if (Variables|Default|GetSpline%20Points%20Placing?)
        (SplineMesh|SetStartandEnd _returnvalue_2 (.Location (Spline|GetLocationandTangentatSplinePoint _spline _output_get "Local")) (Math|Vector|ClampVectorSize (.Tangent (Spline|GetLocationandTangentatSplinePoint _spline _output_get "Local")) 0.0 (Math|Conversions|ToFloat(Integer) (Variables|Default|GetModule%20Width))) (.Location (Spline|GetLocationandTangentatSplinePoint _spline (+ _output_get 1) "Local")) (Math|Vector|ClampVectorSize (.Tangent (Spline|GetLocationandTangentatSplinePoint _spline (+ _output_get 1) "Local")) 0.0 (Math|Conversions|ToFloat(Integer) (Variables|Default|GetModule%20Width))) true :!class /Script/Engine.SplineMeshComponent) ; Spline Points Based
        (Collision|SetCollisionEnabled _returnvalue_2 (Variables|Default|GetCollision%20Type) :!label _label)
        (Transformation|AttachComponentToComponent _returnvalue_2 (Variables|Default|GetDefaultSceneRoot) "None" "KeepRelative" "KeepRelative" "KeepRelative" true)
        ;[1 1 1] Debug
        (Development|PrintString (Utilities|String|ToString(Integer) 0) true true "(R=0.000000,G=0.660000,B=1.000000,A=1.000000)" 5.0)
        (else
          (Utilities|FlowControl|Sequence
            (:then_0
              (SplineMesh|SetStartandEnd _returnvalue_2 (Spline|GetLocationatDistanceAlongSpline _spline_2 (Math|Conversions|ToFloat(Integer) (* (Variables|Default|GetLoop%20Index) (Variables|Default|GetModule%20Width))) "Local") (Math|Vector|ClampVectorSize (Spline|GetTangentatDistanceAlongSpline _spline_2 (Math|Conversions|ToFloat(Integer) (* (Variables|Default|GetLoop%20Index) (Variables|Default|GetModule%20Width))) "Local") 0.0 (Math|Conversions|ToFloat(Integer) (Variables|Default|GetModule%20Width))) (Spline|GetLocationatDistanceAlongSpline _spline_2 (Math|Conversions|ToFloat(Integer) (* (+ (Variables|Default|GetLoop%20Index) 1) (Variables|Default|GetModule%20Width))) "Local") (Math|Vector|ClampVectorSize (Spline|GetTangentatDistanceAlongSpline _spline_2 (Math|Conversions|ToFloat(Integer) (* (+ (Variables|Default|GetLoop%20Index) 1) (Variables|Default|GetModule%20Width))) "Local") 0.0 (Math|Conversions|ToFloat(Integer) (Variables|Default|GetModule%20Width))) true :!class /Script/Engine.SplineMeshComponent) ; Length Based
              (goto _label))
            (:then_1
              (SplineMesh|SetStartandEnd _returnvalue_3 (Spline|GetLocationatDistanceAlongSpline _spline_2 (Math|Conversions|ToFloat(Integer) (* (Variables|Default|GetLoop%20Index) (Variables|Default|GetModule%20Width))) "Local") (Math|Vector|ClampVectorSize (Spline|GetTangentatDistanceAlongSpline _spline_2 (Math|Conversions|ToFloat(Integer) (* (Variables|Default|GetLoop%20Index) (Variables|Default|GetModule%20Width))) "Local") 0.0 (Math|Conversions|ToFloat(Integer) (Variables|Default|GetModule%20Width))) (Spline|GetLocationatDistanceAlongSpline _spline_2 (Math|Conversions|ToFloat(Integer) (* (+ (Variables|Default|GetLoop%20Index) 1) (Variables|Default|GetModule%20Width))) "Local") (Math|Vector|ClampVectorSize (Spline|GetTangentatDistanceAlongSpline _spline_2 (Math|Conversions|ToFloat(Integer) (* (+ (Variables|Default|GetLoop%20Index) 1) (Variables|Default|GetModule%20Width))) "Local") 0.0 (Math|Conversions|ToFloat(Integer) (Variables|Default|GetModule%20Width))) true :!class /Script/Engine.SplineMeshComponent) ; Length Based
            )))))
    (elif (Variables|Default|GetUse%20Full%20Length%20Meshes?) ; Use Full Length Meshes?
      ;[1 1 1] Spline Length Based Indexing. MUST BE FULL LENGTH MESHES
      (for _index_2 (range 0 (- (Math|Float|Truncate (/ (Spline|GetSplineLength (Variables|Default|GetSpline)) (Variables|Default|GetModule%20Width))) 1))
        (Variables|Default|SetLoop%20Index _index_2)
        (bind _returnvalue_4 (AddComponent|AddHierarchicalInstancedStaticMeshComponent true))
        (bind _output_get_3 (Variables|Default|SetHierarchical%20Instanced%20Mesh _returnvalue_4))
        (bind _returnvalue_5 (AddComponent|AddSplineMeshComponent (Components|GetOwner _output_get_3) false))
        (bind _returnvalue_6 (AddComponent|AddSplineMeshComponent (Components|GetOwner _output_get_3) false (Math|Transform|MakeTransform "0.000000,0.000000,300.000000" "0, 0, 0" "1.000000,1.000000,1.000000")))
        (Components|StaticMesh|SetStaticMesh _returnvalue_5 (Utilities|Array|Get(acopy) (.floorelements (Utilities|Array|Get(acopy) _ground_floor_creator (Math|Random|RandomIntegerinRangefromStream 0 (Utilities|Array|LastIndex _ground_floor_creator) (Math|Random|MakeRandomStream (* (Variables|Default|GetInitial%20Random%20Seed) (Variables|Default|GetLoop%20Index)))))))) ; Ground Floor
        (Components|StaticMesh|SetStaticMesh _returnvalue_6 (Utilities|Array|Get(acopy) (.floorelements (Utilities|Array|Get(acopy) _floor_creator (Math|Random|RandomIntegerinRangefromStream 0 (Utilities|Array|LastIndex _floor_creator) (Math|Random|MakeRandomStream (* (Variables|Default|GetInitial%20Random%20Seed) (Variables|Default|GetLoop%20Index)))))))) ; First Floor
        (SplineMesh|SetForwardAxis _returnvalue_5 "X" true)
        (if (Variables|Default|GetSpline%20Points%20Placing?)
          (SplineMesh|SetStartandEnd _returnvalue_5 (.Location (Spline|GetLocationandTangentatSplinePoint _spline _output_get "Local")) (Math|Vector|ClampVectorSize (.Tangent (Spline|GetLocationandTangentatSplinePoint _spline _output_get "Local")) 0.0 (Math|Conversions|ToFloat(Integer) (Variables|Default|GetModule%20Width))) (.Location (Spline|GetLocationandTangentatSplinePoint _spline (+ _output_get 1) "Local")) (Math|Vector|ClampVectorSize (.Tangent (Spline|GetLocationandTangentatSplinePoint _spline (+ _output_get 1) "Local")) 0.0 (Math|Conversions|ToFloat(Integer) (Variables|Default|GetModule%20Width))) true :!class /Script/Engine.SplineMeshComponent) ; Spline Points Based
          (Collision|SetCollisionEnabled _returnvalue_5 (Variables|Default|GetCollision%20Type) :!label _label_2)
          (Transformation|AttachComponentToComponent _returnvalue_5 (Variables|Default|GetDefaultSceneRoot) "None" "KeepRelative" "KeepRelative" "KeepRelative" true)
          (Development|PrintString (Utilities|String|ToString(Integer) 0) true true "(R=0.000000,G=0.660000,B=1.000000,A=1.000000)" 5.0)
          (else
            (Utilities|FlowControl|Sequence
              (:then_0
                (SplineMesh|SetStartandEnd _returnvalue_5 (Spline|GetLocationatDistanceAlongSpline _spline_2 (Math|Conversions|ToFloat(Integer) (* (Variables|Default|GetLoop%20Index) (Variables|Default|GetModule%20Width))) "Local") (Math|Vector|ClampVectorSize (Spline|GetTangentatDistanceAlongSpline _spline_2 (Math|Conversions|ToFloat(Integer) (* (Variables|Default|GetLoop%20Index) (Variables|Default|GetModule%20Width))) "Local") 0.0 (Math|Conversions|ToFloat(Integer) (Variables|Default|GetModule%20Width))) (Spline|GetLocationatDistanceAlongSpline _spline_2 (Math|Conversions|ToFloat(Integer) (* (+ (Variables|Default|GetLoop%20Index) 1) (Variables|Default|GetModule%20Width))) "Local") (Math|Vector|ClampVectorSize (Spline|GetTangentatDistanceAlongSpline _spline_2 (Math|Conversions|ToFloat(Integer) (* (+ (Variables|Default|GetLoop%20Index) 1) (Variables|Default|GetModule%20Width))) "Local") 0.0 (Math|Conversions|ToFloat(Integer) (Variables|Default|GetModule%20Width))) true :!class /Script/Engine.SplineMeshComponent) ; Length Based
                (goto _label_2))
              (:then_1
                (SplineMesh|SetStartandEnd _returnvalue_6 (Spline|GetLocationatDistanceAlongSpline _spline_2 (Math|Conversions|ToFloat(Integer) (* (Variables|Default|GetLoop%20Index) (Variables|Default|GetModule%20Width))) "Local") (Math|Vector|ClampVectorSize (Spline|GetTangentatDistanceAlongSpline _spline_2 (Math|Conversions|ToFloat(Integer) (* (Variables|Default|GetLoop%20Index) (Variables|Default|GetModule%20Width))) "Local") 0.0 (Math|Conversions|ToFloat(Integer) (Variables|Default|GetModule%20Width))) (Spline|GetLocationatDistanceAlongSpline _spline_2 (Math|Conversions|ToFloat(Integer) (* (+ (Variables|Default|GetLoop%20Index) 1) (Variables|Default|GetModule%20Width))) "Local") (Math|Vector|ClampVectorSize (Spline|GetTangentatDistanceAlongSpline _spline_2 (Math|Conversions|ToFloat(Integer) (* (+ (Variables|Default|GetLoop%20Index) 1) (Variables|Default|GetModule%20Width))) "Local") 0.0 (Math|Conversions|ToFloat(Integer) (Variables|Default|GetModule%20Width))) true :!class /Script/Engine.SplineMeshComponent) ; Length Based
              )))))
      (else
        ;[1 1 1] Spline Length Based Indexing. Length/Module Length = Amount of Spline Meshes
        (for _index_3 (range 0 (Math|Float|Truncate (/ (Spline|GetSplineLength (Variables|Default|GetSpline)) (Variables|Default|GetModule%20Width))))
          (Variables|Default|SetLoop%20Index _index_3)
          (bind _returnvalue_7 (AddComponent|AddHierarchicalInstancedStaticMeshComponent true))
          (bind _output_get_4 (Variables|Default|SetHierarchical%20Instanced%20Mesh _returnvalue_7))
          (bind _returnvalue_8 (AddComponent|AddSplineMeshComponent (Components|GetOwner _output_get_4) false))
          (bind _returnvalue_9 (AddComponent|AddSplineMeshComponent (Components|GetOwner _output_get_4) false (Math|Transform|MakeTransform "0.000000,0.000000,300.000000" "0, 0, 0" "1.000000,1.000000,1.000000")))
          (Components|StaticMesh|SetStaticMesh _returnvalue_8 (Utilities|Array|Get(acopy) (.floorelements (Utilities|Array|Get(acopy) _ground_floor_creator (Math|Random|RandomIntegerinRangefromStream 0 (Utilities|Array|LastIndex _ground_floor_creator) (Math|Random|MakeRandomStream (* (Variables|Default|GetInitial%20Random%20Seed) (Variables|Default|GetLoop%20Index)))))))) ; Ground Floor
          (Components|StaticMesh|SetStaticMesh _returnvalue_9 (Utilities|Array|Get(acopy) (.floorelements (Utilities|Array|Get(acopy) _floor_creator (Math|Random|RandomIntegerinRangefromStream 0 (Utilities|Array|LastIndex _floor_creator) (Math|Random|MakeRandomStream (* (Variables|Default|GetInitial%20Random%20Seed) (Variables|Default|GetLoop%20Index)))))))) ; First Floor
          (SplineMesh|SetForwardAxis _returnvalue_8 "X" true)
          (if (Variables|Default|GetSpline%20Points%20Placing?)
            (SplineMesh|SetStartandEnd _returnvalue_8 (.Location (Spline|GetLocationandTangentatSplinePoint _spline _output_get "Local")) (Math|Vector|ClampVectorSize (.Tangent (Spline|GetLocationandTangentatSplinePoint _spline _output_get "Local")) 0.0 (Math|Conversions|ToFloat(Integer) (Variables|Default|GetModule%20Width))) (.Location (Spline|GetLocationandTangentatSplinePoint _spline (+ _output_get 1) "Local")) (Math|Vector|ClampVectorSize (.Tangent (Spline|GetLocationandTangentatSplinePoint _spline (+ _output_get 1) "Local")) 0.0 (Math|Conversions|ToFloat(Integer) (Variables|Default|GetModule%20Width))) true :!class /Script/Engine.SplineMeshComponent) ; Spline Points Based
            (Collision|SetCollisionEnabled _returnvalue_8 (Variables|Default|GetCollision%20Type) :!label _label_3)
            (Transformation|AttachComponentToComponent _returnvalue_8 (Variables|Default|GetDefaultSceneRoot) "None" "KeepRelative" "KeepRelative" "KeepRelative" true)
            (Development|PrintString (Utilities|String|ToString(Integer) 0) true true "(R=0.000000,G=0.660000,B=1.000000,A=1.000000)" 5.0)
            (else
              (Utilities|FlowControl|Sequence
                (:then_0
                  (SplineMesh|SetStartandEnd _returnvalue_8 (Spline|GetLocationatDistanceAlongSpline _spline_2 (Math|Conversions|ToFloat(Integer) (* (Variables|Default|GetLoop%20Index) (Variables|Default|GetModule%20Width))) "Local") (Math|Vector|ClampVectorSize (Spline|GetTangentatDistanceAlongSpline _spline_2 (Math|Conversions|ToFloat(Integer) (* (Variables|Default|GetLoop%20Index) (Variables|Default|GetModule%20Width))) "Local") 0.0 (Math|Conversions|ToFloat(Integer) (Variables|Default|GetModule%20Width))) (Spline|GetLocationatDistanceAlongSpline _spline_2 (Math|Conversions|ToFloat(Integer) (* (+ (Variables|Default|GetLoop%20Index) 1) (Variables|Default|GetModule%20Width))) "Local") (Math|Vector|ClampVectorSize (Spline|GetTangentatDistanceAlongSpline _spline_2 (Math|Conversions|ToFloat(Integer) (* (+ (Variables|Default|GetLoop%20Index) 1) (Variables|Default|GetModule%20Width))) "Local") 0.0 (Math|Conversions|ToFloat(Integer) (Variables|Default|GetModule%20Width))) true :!class /Script/Engine.SplineMeshComponent) ; Length Based
                  (goto _label_3))
                (:then_1
                  (SplineMesh|SetStartandEnd _returnvalue_9 (Spline|GetLocationatDistanceAlongSpline _spline_2 (Math|Conversions|ToFloat(Integer) (* (Variables|Default|GetLoop%20Index) (Variables|Default|GetModule%20Width))) "Local") (Math|Vector|ClampVectorSize (Spline|GetTangentatDistanceAlongSpline _spline_2 (Math|Conversions|ToFloat(Integer) (* (Variables|Default|GetLoop%20Index) (Variables|Default|GetModule%20Width))) "Local") 0.0 (Math|Conversions|ToFloat(Integer) (Variables|Default|GetModule%20Width))) (Spline|GetLocationatDistanceAlongSpline _spline_2 (Math|Conversions|ToFloat(Integer) (* (+ (Variables|Default|GetLoop%20Index) 1) (Variables|Default|GetModule%20Width))) "Local") (Math|Vector|ClampVectorSize (Spline|GetTangentatDistanceAlongSpline _spline_2 (Math|Conversions|ToFloat(Integer) (* (+ (Variables|Default|GetLoop%20Index) 1) (Variables|Default|GetModule%20Width))) "Local") 0.0 (Math|Conversions|ToFloat(Integer) (Variables|Default|GetModule%20Width))) true :!class /Script/Engine.SplineMeshComponent) ; Length Based
                )))))))))