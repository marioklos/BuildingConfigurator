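; Modular building actor that tiles meshes along a spline as hierarchical instanced static meshes, built in the construction script.
; Each RepeatingItemsCreator entry gets its own component and repeats every ModuleWidth, stacked vertically by array index and ModuleHeight.
; Instances combine entry offsets and ModuleRotation with spline location and rotation.
; An unfinished trim test adds components without assigned meshes per module; simple-instancing and material experiments are disconnected.
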(event EventBeginPlay)

(event Collision|EventActorBeginOverlap
  (params (OtherActor :type Actor%20Object%20Reference)))

(event EventTick
  (params (DeltaSeconds :type Float%20%28single-precision%29)))

(fn ConstructionScript
  (bind _spline (Variables|Default|GetSpline))
  ;[0.5 0 0.1167] Structure Based Instancing
  (for (_array_element _array_index) (Variables|Default|GetRepeatingItemsCreator)
    (Variables|Default|SetLoopCount 0) ; Reset Loop Count
    (bind _returnvalue (AddComponent|AddHierarchicalInstancedStaticMeshComponent false))
    (bind _output_get (Variables|Default|SetHierarchical%20Instanced%20Mesh _returnvalue))
    (Components|StaticMesh|SetStaticMesh _output_get (.staticmesh _array_element))
    ;[1 0.7863 0.6661] Spline Setup
    (for _index (range 0 (- (Spline|GetNumberOfSplinePoints _spline) 1))
      (for _index_2 (range 0 (- (Math|Float|Truncate (/ (Math|Vector|Distance(Vector) (Spline|GetLocationatSplinePoint _spline _index "Local") (Spline|GetLocationatSplinePoint _spline (+ _index 1) "Local")) (Variables|Default|GetModule%20Width))) 1))
        (bind _returnvalue_2 (Components|InstancedStaticMesh|AddInstance (Variables|Default|GetHierarchical%20Instanced%20Mesh) (Math|Transform|MakeTransform (Math|Vector|MakeVector (+ (.x (.Location (Math|Transform|BreakTransform (Math|Transform|MakeTransform (.Location (Math|Transform|BreakTransform (Math|Transform|MakeTransform (Math|Vector|MakeVector (.x (.Location (Math|Transform|BreakTransform (.transform _array_element)))) (.y (.Location (Math|Transform|BreakTransform (.transform _array_element)))) (* (+ (.z (.Location (Math|Transform|BreakTransform (.transform _array_element)))) (Variables|Default|GetModule%20Height)) _array_index)) (.Rotation (Math|Transform|BreakTransform (.transform _array_element))) (.Scale (Math|Transform|BreakTransform (.transform _array_element)))))) (Variables|Default|GetModule%20Rotation) (.Scale (Math|Transform|BreakTransform (Math|Transform|MakeTransform (Math|Vector|MakeVector (.x (.Location (Math|Transform|BreakTransform (.transform _array_element)))) (.y (.Location (Math|Transform|BreakTransform (.transform _array_element)))) (* (+ (.z (.Location (Math|Transform|BreakTransform (.transform _array_element)))) (Variables|Default|GetModule%20Height)) _array_index)) (.Rotation (Math|Transform|BreakTransform (.transform _array_element))) (.Scale (Math|Transform|BreakTransform (.transform _array_element)))))))))) (.X (Math|Vector|BreakVector (Spline|GetLocationatDistanceAlongSpline _spline (* (Variables|Default|GetLoopCount) (Variables|Default|GetModule%20Width)) "Local")))) (+ (.y (.Location (Math|Transform|BreakTransform (Math|Transform|MakeTransform (.Location (Math|Transform|BreakTransform (Math|Transform|MakeTransform (Math|Vector|MakeVector (.x (.Location (Math|Transform|BreakTransform (.transform _array_element)))) (.y (.Location (Math|Transform|BreakTransform (.transform _array_element)))) (* (+ (.z (.Location (Math|Transform|BreakTransform (.transform _array_element)))) (Variables|Default|GetModule%20Height)) _array_index)) (.Rotation (Math|Transform|BreakTransform (.transform _array_element))) (.Scale (Math|Transform|BreakTransform (.transform _array_element)))))) (Variables|Default|GetModule%20Rotation) (.Scale (Math|Transform|BreakTransform (Math|Transform|MakeTransform (Math|Vector|MakeVector (.x (.Location (Math|Transform|BreakTransform (.transform _array_element)))) (.y (.Location (Math|Transform|BreakTransform (.transform _array_element)))) (* (+ (.z (.Location (Math|Transform|BreakTransform (.transform _array_element)))) (Variables|Default|GetModule%20Height)) _array_index)) (.Rotation (Math|Transform|BreakTransform (.transform _array_element))) (.Scale (Math|Transform|BreakTransform (.transform _array_element)))))))))) (.Y (Math|Vector|BreakVector (Spline|GetLocationatDistanceAlongSpline _spline (* (Variables|Default|GetLoopCount) (Variables|Default|GetModule%20Width)) "Local")))) (+ (.z (.Location (Math|Transform|BreakTransform (Math|Transform|MakeTransform (.Location (Math|Transform|BreakTransform (Math|Transform|MakeTransform (Math|Vector|MakeVector (.x (.Location (Math|Transform|BreakTransform (.transform _array_element)))) (.y (.Location (Math|Transform|BreakTransform (.transform _array_element)))) (* (+ (.z (.Location (Math|Transform|BreakTransform (.transform _array_element)))) (Variables|Default|GetModule%20Height)) _array_index)) (.Rotation (Math|Transform|BreakTransform (.transform _array_element))) (.Scale (Math|Transform|BreakTransform (.transform _array_element)))))) (Variables|Default|GetModule%20Rotation) (.Scale (Math|Transform|BreakTransform (Math|Transform|MakeTransform (Math|Vector|MakeVector (.x (.Location (Math|Transform|BreakTransform (.transform _array_element)))) (.y (.Location (Math|Transform|BreakTransform (.transform _array_element)))) (* (+ (.z (.Location (Math|Transform|BreakTransform (.transform _array_element)))) (Variables|Default|GetModule%20Height)) _array_index)) (.Rotation (Math|Transform|BreakTransform (.transform _array_element))) (.Scale (Math|Transform|BreakTransform (.transform _array_element)))))))))) (.Z (Math|Vector|BreakVector (Spline|GetLocationatDistanceAlongSpline _spline (* (Variables|Default|GetLoopCount) (Variables|Default|GetModule%20Width)) "Local"))))) (Math|Rotator|MakeRotator (+ (.roll (.Rotation (Math|Transform|BreakTransform (Math|Transform|MakeTransform (.Location (Math|Transform|BreakTransform (Math|Transform|MakeTransform (Math|Vector|MakeVector (.x (.Location (Math|Transform|BreakTransform (.transform _array_element)))) (.y (.Location (Math|Transform|BreakTransform (.transform _array_element)))) (* (+ (.z (.Location (Math|Transform|BreakTransform (.transform _array_element)))) (Variables|Default|GetModule%20Height)) _array_index)) (.Rotation (Math|Transform|BreakTransform (.transform _array_element))) (.Scale (Math|Transform|BreakTransform (.transform _array_element)))))) (Variables|Default|GetModule%20Rotation) (.Scale (Math|Transform|BreakTransform (Math|Transform|MakeTransform (Math|Vector|MakeVector (.x (.Location (Math|Transform|BreakTransform (.transform _array_element)))) (.y (.Location (Math|Transform|BreakTransform (.transform _array_element)))) (* (+ (.z (.Location (Math|Transform|BreakTransform (.transform _array_element)))) (Variables|Default|GetModule%20Height)) _array_index)) (.Rotation (Math|Transform|BreakTransform (.transform _array_element))) (.Scale (Math|Transform|BreakTransform (.transform _array_element)))))))))) (.Roll (Math|Rotator|BreakRotator (Spline|GetRotationatDistanceAlongSpline _spline (* (Variables|Default|GetLoopCount) (Variables|Default|GetModule%20Width)) "Local")))) (+ (.pitch (.Rotation (Math|Transform|BreakTransform (Math|Transform|MakeTransform (.Location (Math|Transform|BreakTransform (Math|Transform|MakeTransform (Math|Vector|MakeVector (.x (.Location (Math|Transform|BreakTransform (.transform _array_element)))) (.y (.Location (Math|Transform|BreakTransform (.transform _array_element)))) (* (+ (.z (.Location (Math|Transform|BreakTransform (.transform _array_element)))) (Variables|Default|GetModule%20Height)) _array_index)) (.Rotation (Math|Transform|BreakTransform (.transform _array_element))) (.Scale (Math|Transform|BreakTransform (.transform _array_element)))))) (Variables|Default|GetModule%20Rotation) (.Scale (Math|Transform|BreakTransform (Math|Transform|MakeTransform (Math|Vector|MakeVector (.x (.Location (Math|Transform|BreakTransform (.transform _array_element)))) (.y (.Location (Math|Transform|BreakTransform (.transform _array_element)))) (* (+ (.z (.Location (Math|Transform|BreakTransform (.transform _array_element)))) (Variables|Default|GetModule%20Height)) _array_index)) (.Rotation (Math|Transform|BreakTransform (.transform _array_element))) (.Scale (Math|Transform|BreakTransform (.transform _array_element)))))))))) (.Pitch (Math|Rotator|BreakRotator (Spline|GetRotationatDistanceAlongSpline _spline (* (Variables|Default|GetLoopCount) (Variables|Default|GetModule%20Width)) "Local")))) (+ (.yaw (.Rotation (Math|Transform|BreakTransform (Math|Transform|MakeTransform (.Location (Math|Transform|BreakTransform (Math|Transform|MakeTransform (Math|Vector|MakeVector (.x (.Location (Math|Transform|BreakTransform (.transform _array_element)))) (.y (.Location (Math|Transform|BreakTransform (.transform _array_element)))) (* (+ (.z (.Location (Math|Transform|BreakTransform (.transform _array_element)))) (Variables|Default|GetModule%20Height)) _array_index)) (.Rotation (Math|Transform|BreakTransform (.transform _array_element))) (.Scale (Math|Transform|BreakTransform (.transform _array_element)))))) (Variables|Default|GetModule%20Rotation) (.Scale (Math|Transform|BreakTransform (Math|Transform|MakeTransform (Math|Vector|MakeVector (.x (.Location (Math|Transform|BreakTransform (.transform _array_element)))) (.y (.Location (Math|Transform|BreakTransform (.transform _array_element)))) (* (+ (.z (.Location (Math|Transform|BreakTransform (.transform _array_element)))) (Variables|Default|GetModule%20Height)) _array_index)) (.Rotation (Math|Transform|BreakTransform (.transform _array_element))) (.Scale (Math|Transform|BreakTransform (.transform _array_element)))))))))) (.Yaw (Math|Rotator|BreakRotator (Spline|GetRotationatDistanceAlongSpline _spline (* (Variables|Default|GetLoopCount) (Variables|Default|GetModule%20Width)) "Local"))))) (.Scale (Math|Transform|BreakTransform (Math|Transform|MakeTransform (.Location (Math|Transform|BreakTransform (Math|Transform|MakeTransform (Math|Vector|MakeVector (.x (.Location (Math|Transform|BreakTransform (.transform _array_element)))) (.y (.Location (Math|Transform|BreakTransform (.transform _array_element)))) (* (+ (.z (.Location (Math|Transform|BreakTransform (.transform _array_element)))) (Variables|Default|GetModule%20Height)) _array_index)) (.Rotation (Math|Transform|BreakTransform (.transform _array_element))) (.Scale (Math|Transform|BreakTransform (.transform _array_element)))))) (Variables|Default|GetModule%20Rotation) (.Scale (Math|Transform|BreakTransform (Math|Transform|MakeTransform (Math|Vector|MakeVector (.x (.Location (Math|Transform|BreakTransform (.transform _array_element)))) (.y (.Location (Math|Transform|BreakTransform (.transform _array_element)))) (* (+ (.z (.Location (Math|Transform|BreakTransform (.transform _array_element)))) (Variables|Default|GetModule%20Height)) _array_index)) (.Rotation (Math|Transform|BreakTransform (.transform _array_element))) (.Scale (Math|Transform|BreakTransform (.transform _array_element)))))))))) false))
        (Math|Integer|IncrementInt (Variables|Default|GetLoopCount)
          (:%20%20
            (for _array_element_2 (Variables|Default|GetRepeatingItemsCreator_TrimTest)
              (bind _returnvalue_3 (AddComponent|AddHierarchicalInstancedStaticMeshComponent false))
              (Components|StaticMesh|SetStaticMesh _returnvalue_3 0)
              (Components|InstancedStaticMesh|AddInstance _returnvalue_3 (.transform _array_element_2) false))))))))