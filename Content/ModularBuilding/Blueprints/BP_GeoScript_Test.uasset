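; Geometry Script test actor that generates a flat polygon mesh from the points of a spline.
; On rebuild it collects local spline points as 2D vertices, appending a raised triangulated polygon from the growing array on each loop pass.
; BakeToStaticMesh copies the dynamic mesh into the MeshTarget asset.
; Unwired experiments cover texture displacement, booleans, remeshing, tessellation, bevels, noise and simplification.
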(event EventBeginPlay)

(event Collision|EventActorBeginOverlap
  (params (OtherActor :type Actor%20Object%20Reference)))

(event EventTick
  (params (DeltaSeconds :type Float%20%28single-precision%29)))

(event Events|EventOnRebuildGeneratedMesh
  (params (TargetMesh :type Dynamic%20Mesh%20Object%20Reference))
  ;[1 0.7629 0] Plane Generator
  (for _index (range 0 (- (Spline|GetNumberOfSplinePoints (Variables|Default|GetSpline)) 1))
    (Utilities|Array|Add (Variables|Default|GetSpline%20Points%20Array) (Math|Conversions|ToVector2D(Vector) (Spline|GetLocationatSplinePoint (Variables|Default|GetSpline) _index "Local")))
    (Class|GeometryScriptLibraryMeshPrimitiveFunctions|AppendTriangulatedPolygon TargetMesh (Utilities|Struct|MakeGeometryScriptPrimitiveOptions "PerFace") (Math|Transform|MakeTransform "0.000000,0.000000,300.000000" "0, 0, 0" "1.000000,1.000000,1.000000") (Variables|Default|GetSpline%20Points%20Array) true 0)))

(fn ConstructionScript
  (Class|GeometryScriptLibraryMeshPrimitiveFunctions|AppendBox :Debug 0))

(fn BaketoStaticMesh
  (bind _meshtarget (Variables|Default|GetMeshTarget)
    (:then
      (bind _returnvalue (DynamicMeshComponent|GetDynamicMesh (Variables|DynamicMeshActor|GetDynamicMeshComponent)))
      (GeometryScript|StaticMesh|CopyMeshtoStaticMesh :FromDynamicMesh _returnvalue :ToStaticMeshAsset _meshtarget :Debug 0))
    (:else)))