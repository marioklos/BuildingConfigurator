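; Modular building actor that builds multi-floor walls along an editable, optionally closed spline in its construction script.
; Each FLOORSEDITOR entry becomes a floor, with module width and height offset derived from mesh bounds.
; Spline meshes either stretch between spline points or repeat by length, with optional spline tangents, spacing and full-length-only pieces.
; Seeded random streams keep each module's mesh pick persistent; BeginPlay and Tick are unused.
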(event EventBeginPlay)

(event Collision|EventActorBeginOverlap
  (params (OtherActor :type Actor%20Object%20Reference)))

(event EventTick
  (params (DeltaSeconds :type Float%20%28single-precision%29)))

(fn ConstructionScript
  (bind _spline (Variables|Default|GetSpline))
  (bind _spline_2 (Variables|Default|GetSpline))
  (bind _spline_3 (Variables|Default|GetSpline))
  (bind _spline_4 (Variables|Default|GetSpline))
  (bind _spline_5 (Variables|Default|GetSpline))
  (bind _returnvalue (Spline|GetNumberOfSplinePoints _spline))
  (bind _returnvalue_2 (Spline|GetTransformatSplinePoint _spline 0 "Local" false))
  (bind _returnvalue_3 (- _returnvalue 1))
  ;[0.6118 0 1] Spline Setup
  (if (Variables|Default|GetClose%20Spline?)
    (switch Utilities|FlowControl|Switch|SwitchonSpline_Switch (Variables|Default|GetClose%20Spline%20Method)
      (:NewEnumerator0
        ;;[1 1 1] ADD Spline Point
        (Spline|AddSplinePointatIndex _spline (.location _returnvalue_2) _returnvalue "Local" true))
      (:NewEnumerator1
        ;;[1 1 1] MOVE Spline Point
        (Spline|SetLocationatSplinePoint _spline _returnvalue_3 (.location _returnvalue_2) "Local" true)
        (Spline|SetRotationatSplinePoint _spline _returnvalue_3 (.rotation _returnvalue_2) "Local" true))))
  (for (_array_element _array_index) (Variables|Default|GetFLOORS%20EDITOR)
    (bind _output_get (Variables|Default|SetFloor%20Elements (.floorelements _array_element)))
    (bind _output_get_2 (Variables|Default|SetFloor%20Random%20Seed (.floorrandomseed _array_element)))
    (Variables|Default|SetSpacing%20Offset (.spacingoffset _array_element))
    ;[0 0.2667 1] Set HEIGHT (automaticly)
    (Variables|Default|SetModule%20Heigth (* (Math|Float|Truncate (.Z (Math|Vector|BreakVector (- (.Max (Utilities|Struct|BreakBox (StaticMesh|GetBoundingBox (CallFunction|RandomMeshfromArray _output_get _output_get_2)))) (.Min (Utilities|Struct|BreakBox (StaticMesh|GetBoundingBox (CallFunction|RandomMeshfromArray _output_get _output_get_2)))))))) _array_index))
    ;[0.1059 1 0] Set WIDTH
    (Variables|Default|SetModule%20Width (Math|Float|Truncate (.X (Math|Vector|BreakVector (- (.Max (Utilities|Struct|BreakBox (StaticMesh|GetBoundingBox (CallFunction|RandomMeshfromArray _output_get _output_get_2)))) (.Min (Utilities|Struct|BreakBox (StaticMesh|GetBoundingBox (CallFunction|RandomMeshfromArray _output_get _output_get_2)))))))))
    (if (Variables|Default|GetAllow%20Scaling?) ; Allow Scaling?
      ;[0.1823 0.05549 0] Scale along the spline
      (Variables|Default|SetModule%20Width (Math|Float|Truncate (* (.x (Transformation|GetActorScale3D)) (Variables|Default|GetModule%20Width)))))
    (if (Variables|Default|GetSpline%20Points%20Placing?%20%28Stretching%29) ; Spline Points
      ;[0.08235 0.08235 0.08235] Spline Points Based Placing
      (for _index (range 0 (- (Spline|GetNumberOfSplinePoints (Variables|Default|GetSpline)) 1))
        ;;[0.06667 0 1] Loop Index
        ;; (for every module)
        (Variables|Default|SetLoop%20Index (* _index (+ (Variables|Default|GetSpacing) (Variables|Default|GetSpacing%20Offset))))
        ;[0.6128 0 1] Setting Up Spline Mesh
        (bind _returnvalue_4 (AddComponent|AddHierarchicalInstancedStaticMeshComponent false))
        (bind _output_get_3 (Variables|Default|SetInstanced%20Mesh%20Actor (Components|GetOwner _returnvalue_4)))
        (if (Variables|Default|GetSpline%20Points%20Placing?%20%28Stretching%29) ; Spline Points
          ;[0.08235 0.08235 0.08235] TANGENT ON; Spline Points Based Placement (STRETCHING)
          (bind _returnvalue_5 (AddComponent|AddSplineMeshComponent (Variables|Default|GetInstanced%20Mesh%20Actor) false (Math|Transform|MakeTransform (Math|Vector|MakeVector 0.0 0.0 (Math|Conversions|ToFloat(Integer) (Variables|Default|GetModule%20Heigth))) "0, 0, 0" "1.000000,1.000000,1.000000")))
          ;;[0.6128 0 1] Setting Up Spline Mesh
          (bind _output_get_4 (Variables|Default|SetSpline%20Mesh _returnvalue_5))
          (Components|StaticMesh|SetStaticMesh _output_get_4 (CallFunction|RandomMeshfromArray (Variables|Default|GetFloor%20Elements) (Variables|Default|GetFloor%20Random%20Seed)))
          (SplineMesh|SetForwardAxis _returnvalue_5 "X" true)
          (if (Variables|Default|GetUse%20Tangent?) ; Spline Points
            (SplineMesh|SetStartandEnd (Variables|Default|GetSpline%20Mesh) (.Location (Spline|GetLocationandTangentatSplinePoint _spline_2 (Variables|Default|GetLoop%20Index) "Local")) (.Tangent (Spline|GetLocationandTangentatSplinePoint _spline_2 (Variables|Default|GetLoop%20Index) "Local")) (.Location (Spline|GetLocationandTangentatSplinePoint _spline_2 (+ (Variables|Default|GetLoop%20Index) 1) "Local")) (.Tangent (Spline|GetLocationandTangentatSplinePoint _spline_2 (+ (Variables|Default|GetLoop%20Index) 1) "Local")) true :!class /Script/Engine.SplineMeshComponent)
            (else
              ;[0.2812 0.2812 0.2812] TANGENT OFF; Spline Points Based Placement (STRETCHING)
              (SplineMesh|SetStartandEnd (Variables|Default|GetSpline%20Mesh) (Spline|GetLocationatSplinePoint _spline_4 (Variables|Default|GetLoop%20Index) "Local") (Math|Vector|ClampVectorSize (Math|Rotator|GetRotationXVector (Math|Rotator|MakeRotfromX (- (Spline|GetLocationatSplinePoint _spline_4 (+ (Variables|Default|GetLoop%20Index) 1) "Local") (Spline|GetLocationatSplinePoint _spline_4 (Variables|Default|GetLoop%20Index) "Local")))) 0.0 (Math|Conversions|ToFloat(Integer) (Variables|Default|GetModule%20Width))) (Spline|GetLocationatSplinePoint _spline_4 (+ (Variables|Default|GetLoop%20Index) 1) "Local") (Math|Vector|ClampVectorSize (Math|Rotator|GetRotationXVector (Math|Rotator|MakeRotfromX (- (Spline|GetLocationatSplinePoint _spline_4 (+ (Variables|Default|GetLoop%20Index) 1) "Local") (Spline|GetLocationatSplinePoint _spline_4 (Variables|Default|GetLoop%20Index) "Local")))) 0.0 (Math|Conversions|ToFloat(Integer) (Variables|Default|GetModule%20Width))) true :!class /Script/Engine.SplineMeshComponent)))
          (elif (Variables|Default|GetUse%20Tangent?) ; Tangent
            ;[0.1059 1 0] Tangent ON
            (bind _returnvalue_6 (AddComponent|AddSplineMeshComponent _output_get_3 false (Math|Transform|MakeTransform (Math|Vector|MakeVector 0.0 0.0 (Math|Conversions|ToFloat(Integer) (Variables|Default|GetModule%20Heigth))) "0, 0, 0" "1.000000,1.000000,1.000000")))
            ;;[0.6128 0 1] Setting Up Spline Mesh
            (bind _output_get_5 (Variables|Default|SetSpline%20Mesh _returnvalue_6))
            (Components|StaticMesh|SetStaticMesh _output_get_5 (CallFunction|RandomMeshfromArray (Variables|Default|GetFloor%20Elements) (Variables|Default|GetFloor%20Random%20Seed))) ; Ground Floor
            ;;[1 0.08235 0.09804] Open up the mesh, look at the pivot point gizmo to determine forward axis
            (SplineMesh|SetForwardAxis _returnvalue_6 "X" true)
            ;[0.1062 1 0] Tangent ON; Length Based Placement +Tangent Rotation
            (SplineMesh|SetStartandEnd (Variables|Default|GetSpline%20Mesh) (Spline|GetLocationatDistanceAlongSpline _spline_5 (Math|Conversions|ToFloat(Integer) (* (Variables|Default|GetLoop%20Index) (Variables|Default|GetModule%20Width))) "Local") (Math|Rotator|GetRotationXVector (Math|Conversions|RotationFromXVector (Math|Vector|ClampVectorSize (Spline|GetTangentatDistanceAlongSpline _spline_5 (Math|Conversions|ToFloat(Integer) (* (Variables|Default|GetLoop%20Index) (Variables|Default|GetModule%20Width))) "Local") 0.0 (Math|Conversions|ToFloat(Integer) (Variables|Default|GetModule%20Width))))) (Spline|GetLocationatDistanceAlongSpline _spline_5 (Math|Conversions|ToFloat(Integer) (* (+ (Variables|Default|GetLoop%20Index) 1) (Variables|Default|GetModule%20Width))) "Local") (Math|Rotator|GetRotationXVector (Math|Conversions|RotationFromXVector (Math|Vector|ClampVectorSize (Spline|GetTangentatDistanceAlongSpline _spline_5 (Math|Conversions|ToFloat(Integer) (* (+ (Variables|Default|GetLoop%20Index) 1) (Variables|Default|GetModule%20Width))) "Local") 0.0 (Math|Conversions|ToFloat(Integer) (Variables|Default|GetModule%20Width))))) true :!class /Script/Engine.SplineMeshComponent) ; Length Based
            (else
              ;[0 1 0.6928] Tangent OFF
              (bind _returnvalue_7 (AddComponent|AddSplineMeshComponent _output_get_3 false (Math|Transform|MakeTransform (Math|Vector|MakeVector 0.0 0.0 (Math|Conversions|ToFloat(Integer) (Variables|Default|GetModule%20Heigth))) "0, 0, 0" "1.000000,1.000000,1.000000")))
              ;;[0.6128 0 1] Setting Up Spline Mesh
              (bind _output_get_6 (Variables|Default|SetSpline%20Mesh _returnvalue_7))
              (Components|StaticMesh|SetStaticMesh _output_get_6 (CallFunction|RandomMeshfromArray (Variables|Default|GetFloor%20Elements) (Variables|Default|GetFloor%20Random%20Seed))) ; Ground Floor
              ;;[1 0.08235 0.09804] Open up the mesh, look at the pivot point gizmo to determine forward axis
              (SplineMesh|SetForwardAxis _returnvalue_7 "X" true)
              ;[0 1 0.6928] Tangent OFF
              (SplineMesh|SetStartandEnd (Variables|Default|GetSpline%20Mesh) (Spline|GetLocationatDistanceAlongSpline _spline_3 (Math|Conversions|ToFloat(Integer) (* (Variables|Default|GetLoop%20Index) (Variables|Default|GetModule%20Width))) "Local") (Math|Vector|ClampVectorSize (Math|Rotator|GetRotationXVector (Math|Rotator|MakeRotfromX (- (Spline|GetLocationatDistanceAlongSpline _spline_3 (Math|Conversions|ToFloat(Integer) (* (+ (Variables|Default|GetLoop%20Index) 1) (Variables|Default|GetModule%20Width))) "Local") (Spline|GetLocationatDistanceAlongSpline _spline_3 (Math|Conversions|ToFloat(Integer) (* (Variables|Default|GetLoop%20Index) (Variables|Default|GetModule%20Width))) "Local")))) 0.0 (Math|Conversions|ToFloat(Integer) (Variables|Default|GetModule%20Width))) (Spline|GetLocationatDistanceAlongSpline _spline_3 (Math|Conversions|ToFloat(Integer) (* (+ (Variables|Default|GetLoop%20Index) 1) (Variables|Default|GetModule%20Width))) "Local") (Math|Vector|ClampVectorSize (Math|Rotator|GetRotationXVector (Math|Rotator|MakeRotfromX (- (Spline|GetLocationatDistanceAlongSpline _spline_3 (Math|Conversions|ToFloat(Integer) (* (+ (Variables|Default|GetLoop%20Index) 1) (Variables|Default|GetModule%20Width))) "Local") (Spline|GetLocationatDistanceAlongSpline _spline_3 (Math|Conversions|ToFloat(Integer) (* (Variables|Default|GetLoop%20Index) (Variables|Default|GetModule%20Width))) "Local")))) 0.0 (Math|Conversions|ToFloat(Integer) (Variables|Default|GetModule%20Width))) true :!class /Script/Engine.SplineMeshComponent))))
        (Collision|SetCollisionEnabled (Variables|Default|GetSpline%20Mesh) (Variables|Default|GetCollision%20Type))
        (Transformation|AttachComponentToComponent (Variables|Default|GetSpline%20Mesh) (Variables|Default|GetDefaultSceneRoot) "None" "KeepRelative" "KeepRelative" "KeepRelative" true))
      (elif (Variables|Default|GetUse%20Full%20Length%20Meshes?) ; Use Full Length Meshes?
        ;[1 0.2153 0] Spline Length Based Indexing. MUST BE FULL LENGTH MESHES
        (for _index_2 (range 0 (- (Math|Float|Floor (/ (Spline|GetSplineLength (Variables|Default|GetSpline)) (Variables|Default|GetModule%20Width))) 1))
          ;;[0.06667 0 1] Loop Index
          ;; (for every module)
          (Variables|Default|SetLoop%20Index (* (+ (Variables|Default|GetSpacing) (Variables|Default|GetSpacing%20Offset)) _index_2))
          (bind _returnvalue_8 (AddComponent|AddHierarchicalInstancedStaticMeshComponent false))
          (bind _output_get_7 (Variables|Default|SetInstanced%20Mesh%20Actor (Components|GetOwner _returnvalue_8)))
          (if (Variables|Default|GetSpline%20Points%20Placing?%20%28Stretching%29) ; Spline Points
            (bind _returnvalue_9 (AddComponent|AddSplineMeshComponent (Variables|Default|GetInstanced%20Mesh%20Actor) false (Math|Transform|MakeTransform (Math|Vector|MakeVector 0.0 0.0 (Math|Conversions|ToFloat(Integer) (Variables|Default|GetModule%20Heigth))) "0, 0, 0" "1.000000,1.000000,1.000000")))
            (bind _output_get_8 (Variables|Default|SetSpline%20Mesh _returnvalue_9))
            (Components|StaticMesh|SetStaticMesh _output_get_8 (CallFunction|RandomMeshfromArray (Variables|Default|GetFloor%20Elements) (Variables|Default|GetFloor%20Random%20Seed)))
            (SplineMesh|SetForwardAxis _returnvalue_9 "X" true)
            (if (Variables|Default|GetUse%20Tangent?) ; Spline Points
              (SplineMesh|SetStartandEnd (Variables|Default|GetSpline%20Mesh) (.Location (Spline|GetLocationandTangentatSplinePoint _spline_2 (Variables|Default|GetLoop%20Index) "Local")) (.Tangent (Spline|GetLocationandTangentatSplinePoint _spline_2 (Variables|Default|GetLoop%20Index) "Local")) (.Location (Spline|GetLocationandTangentatSplinePoint _spline_2 (+ (Variables|Default|GetLoop%20Index) 1) "Local")) (.Tangent (Spline|GetLocationandTangentatSplinePoint _spline_2 (+ (Variables|Default|GetLoop%20Index) 1) "Local")) true :!class /Script/Engine.SplineMeshComponent)
              (else
                (SplineMesh|SetStartandEnd (Variables|Default|GetSpline%20Mesh) (Spline|GetLocationatSplinePoint _spline_4 (Variables|Default|GetLoop%20Index) "Local") (Math|Vector|ClampVectorSize (Math|Rotator|GetRotationXVector (Math|Rotator|MakeRotfromX (- (Spline|GetLocationatSplinePoint _spline_4 (+ (Variables|Default|GetLoop%20Index) 1) "Local") (Spline|GetLocationatSplinePoint _spline_4 (Variables|Default|GetLoop%20Index) "Local")))) 0.0 (Math|Conversions|ToFloat(Integer) (Variables|Default|GetModule%20Width))) (Spline|GetLocationatSplinePoint _spline_4 (+ (Variables|Default|GetLoop%20Index) 1) "Local") (Math|Vector|ClampVectorSize (Math|Rotator|GetRotationXVector (Math|Rotator|MakeRotfromX (- (Spline|GetLocationatSplinePoint _spline_4 (+ (Variables|Default|GetLoop%20Index) 1) "Local") (Spline|GetLocationatSplinePoint _spline_4 (Variables|Default|GetLoop%20Index) "Local")))) 0.0 (Math|Conversions|ToFloat(Integer) (Variables|Default|GetModule%20Width))) true :!class /Script/Engine.SplineMeshComponent)))
            (elif (Variables|Default|GetUse%20Tangent?) ; Tangent
              (bind _returnvalue_10 (AddComponent|AddSplineMeshComponent _output_get_7 false (Math|Transform|MakeTransform (Math|Vector|MakeVector 0.0 0.0 (Math|Conversions|ToFloat(Integer) (Variables|Default|GetModule%20Heigth))) "0, 0, 0" "1.000000,1.000000,1.000000")))
              (bind _output_get_9 (Variables|Default|SetSpline%20Mesh _returnvalue_10))
              (Components|StaticMesh|SetStaticMesh _output_get_9 (CallFunction|RandomMeshfromArray (Variables|Default|GetFloor%20Elements) (Variables|Default|GetFloor%20Random%20Seed))) ; Ground Floor
              (SplineMesh|SetForwardAxis _returnvalue_10 "X" true)
              (SplineMesh|SetStartandEnd (Variables|Default|GetSpline%20Mesh) (Spline|GetLocationatDistanceAlongSpline _spline_5 (Math|Conversions|ToFloat(Integer) (* (Variables|Default|GetLoop%20Index) (Variables|Default|GetModule%20Width))) "Local") (Math|Rotator|GetRotationXVector (Math|Conversions|RotationFromXVector (Math|Vector|ClampVectorSize (Spline|GetTangentatDistanceAlongSpline _spline_5 (Math|Conversions|ToFloat(Integer) (* (Variables|Default|GetLoop%20Index) (Variables|Default|GetModule%20Width))) "Local") 0.0 (Math|Conversions|ToFloat(Integer) (Variables|Default|GetModule%20Width))))) (Spline|GetLocationatDistanceAlongSpline _spline_5 (Math|Conversions|ToFloat(Integer) (* (+ (Variables|Default|GetLoop%20Index) 1) (Variables|Default|GetModule%20Width))) "Local") (Math|Rotator|GetRotationXVector (Math|Conversions|RotationFromXVector (Math|Vector|ClampVectorSize (Spline|GetTangentatDistanceAlongSpline _spline_5 (Math|Conversions|ToFloat(Integer) (* (+ (Variables|Default|GetLoop%20Index) 1) (Variables|Default|GetModule%20Width))) "Local") 0.0 (Math|Conversions|ToFloat(Integer) (Variables|Default|GetModule%20Width))))) true :!class /Script/Engine.SplineMeshComponent) ; Length Based
              (else
                (bind _returnvalue_11 (AddComponent|AddSplineMeshComponent _output_get_7 false (Math|Transform|MakeTransform (Math|Vector|MakeVector 0.0 0.0 (Math|Conversions|ToFloat(Integer) (Variables|Default|GetModule%20Heigth))) "0, 0, 0" "1.000000,1.000000,1.000000")))
                (bind _output_get_10 (Variables|Default|SetSpline%20Mesh _returnvalue_11))
                (Components|StaticMesh|SetStaticMesh _output_get_10 (CallFunction|RandomMeshfromArray (Variables|Default|GetFloor%20Elements) (Variables|Default|GetFloor%20Random%20Seed))) ; Ground Floor
                (SplineMesh|SetForwardAxis _returnvalue_11 "X" true)
                (SplineMesh|SetStartandEnd (Variables|Default|GetSpline%20Mesh) (Spline|GetLocationatDistanceAlongSpline _spline_3 (Math|Conversions|ToFloat(Integer) (* (Variables|Default|GetLoop%20Index) (Variables|Default|GetModule%20Width))) "Local") (Math|Vector|ClampVectorSize (Math|Rotator|GetRotationXVector (Math|Rotator|MakeRotfromX (- (Spline|GetLocationatDistanceAlongSpline _spline_3 (Math|Conversions|ToFloat(Integer) (* (+ (Variables|Default|GetLoop%20Index) 1) (Variables|Default|GetModule%20Width))) "Local") (Spline|GetLocationatDistanceAlongSpline _spline_3 (Math|Conversions|ToFloat(Integer) (* (Variables|Default|GetLoop%20Index) (Variables|Default|GetModule%20Width))) "Local")))) 0.0 (Math|Conversions|ToFloat(Integer) (Variables|Default|GetModule%20Width))) (Spline|GetLocationatDistanceAlongSpline _spline_3 (Math|Conversions|ToFloat(Integer) (* (+ (Variables|Default|GetLoop%20Index) 1) (Variables|Default|GetModule%20Width))) "Local") (Math|Vector|ClampVectorSize (Math|Rotator|GetRotationXVector (Math|Rotator|MakeRotfromX (- (Spline|GetLocationatDistanceAlongSpline _spline_3 (Math|Conversions|ToFloat(Integer) (* (+ (Variables|Default|GetLoop%20Index) 1) (Variables|Default|GetModule%20Width))) "Local") (Spline|GetLocationatDistanceAlongSpline _spline_3 (Math|Conversions|ToFloat(Integer) (* (Variables|Default|GetLoop%20Index) (Variables|Default|GetModule%20Width))) "Local")))) 0.0 (Math|Conversions|ToFloat(Integer) (Variables|Default|GetModule%20Width))) true :!class /Script/Engine.SplineMeshComponent))))
          (Collision|SetCollisionEnabled (Variables|Default|GetSpline%20Mesh) (Variables|Default|GetCollision%20Type))
          (Transformation|AttachComponentToComponent (Variables|Default|GetSpline%20Mesh) (Variables|Default|GetDefaultSceneRoot) "None" "KeepRelative" "KeepRelative" "KeepRelative" true))
        (else
          ;[1 0.4428 0] Spline Length Based Indexing. Length/Module Length = Amount of Spline Meshes
          (for _index_3 (range 0 (Math|Float|Floor (/ (Spline|GetSplineLength (Variables|Default|GetSpline)) (Variables|Default|GetModule%20Width))))
            ;;[0.06667 0 1] Loop Index
            ;; (for every module)
            (Variables|Default|SetLoop%20Index (* _index_3 (+ (Variables|Default|GetSpacing) (Variables|Default|GetSpacing%20Offset))))
            (bind _returnvalue_12 (AddComponent|AddHierarchicalInstancedStaticMeshComponent false))
            (bind _output_get_11 (Variables|Default|SetInstanced%20Mesh%20Actor (Components|GetOwner _returnvalue_12)))
            (if (Variables|Default|GetSpline%20Points%20Placing?%20%28Stretching%29) ; Spline Points
              (bind _returnvalue_13 (AddComponent|AddSplineMeshComponent (Variables|Default|GetInstanced%20Mesh%20Actor) false (Math|Transform|MakeTransform (Math|Vector|MakeVector 0.0 0.0 (Math|Conversions|ToFloat(Integer) (Variables|Default|GetModule%20Heigth))) "0, 0, 0" "1.000000,1.000000,1.000000")))
              (bind _output_get_12 (Variables|Default|SetSpline%20Mesh _returnvalue_13))
              (Components|StaticMesh|SetStaticMesh _output_get_12 (CallFunction|RandomMeshfromArray (Variables|Default|GetFloor%20Elements) (Variables|Default|GetFloor%20Random%20Seed)))
              (SplineMesh|SetForwardAxis _returnvalue_13 "X" true)
              (if (Variables|Default|GetUse%20Tangent?) ; Spline Points
                (SplineMesh|SetStartandEnd (Variables|Default|GetSpline%20Mesh) (.Location (Spline|GetLocationandTangentatSplinePoint _spline_2 (Variables|Default|GetLoop%20Index) "Local")) (.Tangent (Spline|GetLocationandTangentatSplinePoint _spline_2 (Variables|Default|GetLoop%20Index) "Local")) (.Location (Spline|GetLocationandTangentatSplinePoint _spline_2 (+ (Variables|Default|GetLoop%20Index) 1) "Local")) (.Tangent (Spline|GetLocationandTangentatSplinePoint _spline_2 (+ (Variables|Default|GetLoop%20Index) 1) "Local")) true :!class /Script/Engine.SplineMeshComponent)
                (else
                  (SplineMesh|SetStartandEnd (Variables|Default|GetSpline%20Mesh) (Spline|GetLocationatSplinePoint _spline_4 (Variables|Default|GetLoop%20Index) "Local") (Math|Vector|ClampVectorSize (Math|Rotator|GetRotationXVector (Math|Rotator|MakeRotfromX (- (Spline|GetLocationatSplinePoint _spline_4 (+ (Variables|Default|GetLoop%20Index) 1) "Local") (Spline|GetLocationatSplinePoint _spline_4 (Variables|Default|GetLoop%20Index) "Local")))) 0.0 (Math|Conversions|ToFloat(Integer) (Variables|Default|GetModule%20Width))) (Spline|GetLocationatSplinePoint _spline_4 (+ (Variables|Default|GetLoop%20Index) 1) "Local") (Math|Vector|ClampVectorSize (Math|Rotator|GetRotationXVector (Math|Rotator|MakeRotfromX (- (Spline|GetLocationatSplinePoint _spline_4 (+ (Variables|Default|GetLoop%20Index) 1) "Local") (Spline|GetLocationatSplinePoint _spline_4 (Variables|Default|GetLoop%20Index) "Local")))) 0.0 (Math|Conversions|ToFloat(Integer) (Variables|Default|GetModule%20Width))) true :!class /Script/Engine.SplineMeshComponent)))
              (elif (Variables|Default|GetUse%20Tangent?) ; Tangent
                (bind _returnvalue_14 (AddComponent|AddSplineMeshComponent _output_get_11 false (Math|Transform|MakeTransform (Math|Vector|MakeVector 0.0 0.0 (Math|Conversions|ToFloat(Integer) (Variables|Default|GetModule%20Heigth))) "0, 0, 0" "1.000000,1.000000,1.000000")))
                (bind _output_get_13 (Variables|Default|SetSpline%20Mesh _returnvalue_14))
                (Components|StaticMesh|SetStaticMesh _output_get_13 (CallFunction|RandomMeshfromArray (Variables|Default|GetFloor%20Elements) (Variables|Default|GetFloor%20Random%20Seed))) ; Ground Floor
                (SplineMesh|SetForwardAxis _returnvalue_14 "X" true)
                (SplineMesh|SetStartandEnd (Variables|Default|GetSpline%20Mesh) (Spline|GetLocationatDistanceAlongSpline _spline_5 (Math|Conversions|ToFloat(Integer) (* (Variables|Default|GetLoop%20Index) (Variables|Default|GetModule%20Width))) "Local") (Math|Rotator|GetRotationXVector (Math|Conversions|RotationFromXVector (Math|Vector|ClampVectorSize (Spline|GetTangentatDistanceAlongSpline _spline_5 (Math|Conversions|ToFloat(Integer) (* (Variables|Default|GetLoop%20Index) (Variables|Default|GetModule%20Width))) "Local") 0.0 (Math|Conversions|ToFloat(Integer) (Variables|Default|GetModule%20Width))))) (Spline|GetLocationatDistanceAlongSpline _spline_5 (Math|Conversions|ToFloat(Integer) (* (+ (Variables|Default|GetLoop%20Index) 1) (Variables|Default|GetModule%20Width))) "Local") (Math|Rotator|GetRotationXVector (Math|Conversions|RotationFromXVector (Math|Vector|ClampVectorSize (Spline|GetTangentatDistanceAlongSpline _spline_5 (Math|Conversions|ToFloat(Integer) (* (+ (Variables|Default|GetLoop%20Index) 1) (Variables|Default|GetModule%20Width))) "Local") 0.0 (Math|Conversions|ToFloat(Integer) (Variables|Default|GetModule%20Width))))) true :!class /Script/Engine.SplineMeshComponent) ; Length Based
                (else
                  (bind _returnvalue_15 (AddComponent|AddSplineMeshComponent _output_get_11 false (Math|Transform|MakeTransform (Math|Vector|MakeVector 0.0 0.0 (Math|Conversions|ToFloat(Integer) (Variables|Default|GetModule%20Heigth))) "0, 0, 0" "1.000000,1.000000,1.000000")))
                  (bind _output_get_14 (Variables|Default|SetSpline%20Mesh _returnvalue_15))
                  (Components|StaticMesh|SetStaticMesh _output_get_14 (CallFunction|RandomMeshfromArray (Variables|Default|GetFloor%20Elements) (Variables|Default|GetFloor%20Random%20Seed))) ; Ground Floor
                  (SplineMesh|SetForwardAxis _returnvalue_15 "X" true)
                  (SplineMesh|SetStartandEnd (Variables|Default|GetSpline%20Mesh) (Spline|GetLocationatDistanceAlongSpline _spline_3 (Math|Conversions|ToFloat(Integer) (* (Variables|Default|GetLoop%20Index) (Variables|Default|GetModule%20Width))) "Local") (Math|Vector|ClampVectorSize (Math|Rotator|GetRotationXVector (Math|Rotator|MakeRotfromX (- (Spline|GetLocationatDistanceAlongSpline _spline_3 (Math|Conversions|ToFloat(Integer) (* (+ (Variables|Default|GetLoop%20Index) 1) (Variables|Default|GetModule%20Width))) "Local") (Spline|GetLocationatDistanceAlongSpline _spline_3 (Math|Conversions|ToFloat(Integer) (* (Variables|Default|GetLoop%20Index) (Variables|Default|GetModule%20Width))) "Local")))) 0.0 (Math|Conversions|ToFloat(Integer) (Variables|Default|GetModule%20Width))) (Spline|GetLocationatDistanceAlongSpline _spline_3 (Math|Conversions|ToFloat(Integer) (* (+ (Variables|Default|GetLoop%20Index) 1) (Variables|Default|GetModule%20Width))) "Local") (Math|Vector|ClampVectorSize (Math|Rotator|GetRotationXVector (Math|Rotator|MakeRotfromX (- (Spline|GetLocationatDistanceAlongSpline _spline_3 (Math|Conversions|ToFloat(Integer) (* (+ (Variables|Default|GetLoop%20Index) 1) (Variables|Default|GetModule%20Width))) "Local") (Spline|GetLocationatDistanceAlongSpline _spline_3 (Math|Conversions|ToFloat(Integer) (* (Variables|Default|GetLoop%20Index) (Variables|Default|GetModule%20Width))) "Local")))) 0.0 (Math|Conversions|ToFloat(Integer) (Variables|Default|GetModule%20Width))) true :!class /Script/Engine.SplineMeshComponent))))
            (Collision|SetCollisionEnabled (Variables|Default|GetSpline%20Mesh) (Variables|Default|GetCollision%20Type))
            (Transformation|AttachComponentToComponent (Variables|Default|GetSpline%20Mesh) (Variables|Default|GetDefaultSceneRoot) "None" "KeepRelative" "KeepRelative" "KeepRelative" true)))))))

(fn GetLocationandIndexatDistance
  (params (Loop%20Index :type Integer))
  (return (Spline|GetLocationatDistanceAlongSpline (Variables|Default|GetSpline) (* Loop%20Index (Variables|Default|GetModule%20Width)) "Local")))

(fn RandomMeshfromArray
  (params (Mesh%20Array :type Array%20of%20Static%20Mesh%20Object%20References) (Floor%20Random%20Seed :type Integer))
  (return (Utilities|Array|Get(acopy) Mesh%20Array (Math|Random|RandomIntegerinRangefromStream 0 (Utilities|Array|LastIndex Mesh%20Array) (Math|Random|MakeRandomStream (* (+ Floor%20Random%20Seed (Variables|Default|GetGlobal%20Random%20Seed)) (Variables|Default|GetLoop%20Index)))))))