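; Procedural modular wall actor, apparently for ground floors (GF), that builds a row of static mesh modules in its construction script.
; Module count is either set directly or derived from the EndPoint handle's distance divided by ModuleWidth; the handle's direction is unused.
; Each module is a separate component offset along local Y, its mesh picked from GFMeshArray using InitialRandomSeed times index for persistent variation.
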(event EventBeginPlay)

(event Collision|EventActorBeginOverlap
  (params (OtherActor :type Actor%20Object%20Reference)))

(event EventTick
  (params (DeltaSeconds :type Float%20%28single-precision%29)))

(fn ConstructionScript
  (bind _gf_mesh_array (Variables|Default|GetGF_Mesh_Array))
  (if (Variables|Default|GetUse_End_Point_Handle)
    (bind _output_get (Variables|Default|SetNumber%20of%20Attached%20Modules (Math|Float|Floor (/ (Math|Vector|VectorLength (Variables|Default|GetEndPoint)) (Variables|Default|GetModule%20Width)))))
    (else
      (Variables|Default|SetNumber%20of%20Attached%20Modules (Variables|Default|GetNumber%20of%20Attached%20Modules))))
  (for _index (range 0 _output_get)
    (bind _returnvalue (AddComponent|AddStaticMeshComponent false (Math|Transform|MakeTransform (Math|Vector|MakeVector 0.0 (Math|Conversions|ToFloat(Integer) (* _index (Variables|Default|GetModule%20Width))) 0.0) "0, 0, 0" "1.000000,1.000000,1.000000")))
    (Components|StaticMesh|SetStaticMesh _returnvalue (Utilities|Array|Get(acopy) _gf_mesh_array (Math|Random|RandomIntegerinRangefromStream 0 (Utilities|Array|LastIndex _gf_mesh_array) (Math|Random|MakeRandomStream (* (Variables|Default|GetInitial%20Random%20Seed) _index)))))))