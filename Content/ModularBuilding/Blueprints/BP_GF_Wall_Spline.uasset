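; Modular building actor that lays GF wall modules along an editable spline in its construction script.
; It adds a Y-forward spline mesh component for each ModuleWidth step along the spline, including one for any final remainder.
; Start and end tangents are clamped to the module width to avoid scaling issues.
; Each segment picks its mesh from GFMeshArray using a stream seeded by InitialRandomSeed times its index, so variation persists across rebuilds.
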(event EventBeginPlay)

(event Collision|EventActorBeginOverlap
  (params (OtherActor :type Actor%20Object%20Reference)))

(event EventTick
  (params (DeltaSeconds :type Float%20%28single-precision%29)))

(fn ConstructionScript
  (bind _spline (Variables|Default|GetSpline))
  (bind _gf_mesh_array (Variables|Default|GetGF%20Mesh%20Array))
  ;[1 1 1] Spline Length Based Indexing
  (for _index (range 0 (Math|Float|Floor (/ (Spline|GetSplineLength (Variables|Default|GetSpline)) (Variables|Default|GetModule%20Width))))
    (bind _returnvalue (AddComponent|AddSplineMeshComponent false))
    (SplineMesh|SetForwardAxis _returnvalue "Y" true)
    (SplineMesh|SetStartandEnd _returnvalue (Spline|GetLocationatDistanceAlongSpline _spline (Math|Conversions|ToFloat(Integer) (* _index (Variables|Default|GetModule%20Width))) "Local") (Math|Vector|ClampVectorSize (Spline|GetTangentatDistanceAlongSpline _spline (Math|Conversions|ToFloat(Integer) (* _index (Variables|Default|GetModule%20Width))) "Local") 0.0 (Math|Conversions|ToFloat(Integer) (Variables|Default|GetModule%20Width))) (Spline|GetLocationatDistanceAlongSpline _spline (Math|Conversions|ToFloat(Integer) (* (+ _index 1) (Variables|Default|GetModule%20Width))) "Local") (Math|Vector|ClampVectorSize (Spline|GetTangentatDistanceAlongSpline _spline (Math|Conversions|ToFloat(Integer) (* (+ _index 1) (Variables|Default|GetModule%20Width))) "Local") 0.0 (Math|Conversions|ToFloat(Integer) (Variables|Default|GetModule%20Width))) true :!class /Script/Engine.SplineMeshComponent)
    (Components|StaticMesh|SetStaticMesh _returnvalue (Utilities|Array|Get(acopy) _gf_mesh_array (Math|Random|RandomIntegerinRangefromStream 0 (Utilities|Array|LastIndex _gf_mesh_array) (Math|Random|MakeRandomStream (* (Variables|Default|GetInitial%20Random%20Seed) _index)))))))